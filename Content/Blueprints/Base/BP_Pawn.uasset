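; First-person pawn that moves, looks, shows a crosshair and lets the player inspect world items tagged Interactable.
; A camera trace each tick highlights targets through custom depth stencil.
; LMB press swaps the target for a ChildActor copy animated toward ViewPosition, and RMB starts inspection on that BP_Inspect_Device.
; LMB release or EndInteract reverses the animation, respawns the item and lerps it back to its original transform.
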(event Custom|End%20Interact
  (bind _camera (Variables|Default|GetCamera))
  (bind _itemactor (Variables|Default|GetItemActor))
  (bind _returnvalue (Transformation|GetWorldTransform _camera))
  ;[1 1 1] LMB Interact
  (if (Variables|Default|GetInspecting?)
    ;;[1 1 1] LMB released
    ;;;[1 1 1] reset rotation lock while timeline is active
    (bind _asbp_inspect_device (Utilities|Casting|CastToBP_Inspect_Device (Variables|/Script/Engine.ChildActorComponent|GetChildActor (Variables|Default|GetItemActor))))
    (Variables|/Game/Blueprints/Interactables/BP_Inspect_Device.BP_Inspect_Device_C|SetinFocus? _asbp_inspect_device false)
    ;;;[1 1 1] Show HUD after release
    (Default|ShowHUD _asbp_inspect_device)
    ;;;[1 1 1] Reverse pick up animation
    (bind _item_track (Timeline|Timeline_3 Reverse)
      (:Update
        (Variables|Default|SetStartLocationTrs (Transformation|GetRelativeTransform (Variables|Default|GetItemActor)))
        (Variables|Default|SetEndLocationTrs (Transformation|GetRelativeTransform (Variables|Default|GetView_Position)))
        (Transformation|SetRelativeTransform (Variables|Default|GetItemActor) (Math|Transform|Lerp(Transform) (Variables|Default|GetStartLocationTrs) (Variables|Default|GetEndLocationTrs) _item_track) false false))
      (:Finished
        ;;;[1 1 1] Spawns the held item back into the world
        (bind _returnvalue_2 (Game|SpawnActorfromClass (Variables|/Script/Engine.ChildActorComponent|GetChildActorClass (Variables|Default|GetItemActor)) (Math|Transform|MakeTransform (Math|Transform|TransformLocation _returnvalue (Variables|/Script/Engine.SceneComponent|GetRelativeLocation _itemactor)) (Math|Transform|TransformRotation _returnvalue (Variables|/Script/Engine.SceneComponent|GetRelativeRotation _itemactor))) "Undefined" 0 0))
        (Variables|Default|SetPlacedItem _returnvalue_2)
        ;;;[1 1 1] removes item holding
        (ChildActorComponent|SetChildActorClass (Variables|Default|GetItemActor) 0)
        ;;;[1 1 1] Sets the item transform as start location
        (Variables|Default|SetReturnStartLocationTrs (Transformation|GetActorTransform (Variables|Default|GetPlacedItem)))
        ;;;[1 1 1] Place down animation
        (bind _return_location_track (Timeline|Reset%20item%20location PlayFromStart)
          (:Update
            (Transformation|SetActorTransform (Variables|Default|GetPlacedItem) (Math|Transform|Lerp(Transform) (Variables|Default|GetReturnStartLocationTrs) (Variables|Default|GetReturnEndLocationTrs) _return_location_track)))
          (:Finished
            (Variables|Default|SetInspecting? false)))))))

(event EventTick
  (params (DeltaSeconds :type Float%20%28single-precision%29))
  (bind _camera (Variables|Default|GetCamera))
  (bind _returnvalue (Transformation|GetWorldLocation _camera))
  ;[1 1 1] Event Tick
  (bind (_outhit _returnvalue_2) (Collision|LineTraceByChannel _returnvalue (+ _returnvalue (* (Math|Vector|GetForwardVector _camera) 1000)) "TraceTypeQuery1" false 0 "None"))
  (if _returnvalue_2
    (if (Actor|ActorHasTag (.HitActor (Collision|BreakHitResult _outhit)) "Interactable")
      ;;[1 1 1] Prevent highlight while inspecting
      (if (not (Variables|Default|GetInspecting?))
        ;;[1 1 1] Highlight device
        (Rendering|SetRenderCustomDepth (.HitComponent (Collision|BreakHitResult _outhit)) true)
        (Rendering|SetCustomDepthStencilValue (.HitComponent (Collision|BreakHitResult _outhit)) 10)
        (Variables|Default|SetOldMesh (.HitComponent (Collision|BreakHitResult _outhit))))
      (else
        ;;[1 1 1] Clear highlight
        (Utilities|IsValid (Variables|Default|GetOldMesh)
          (:Is%20Valid
            (CallFunction|ClearHighlight (Variables|Default|GetOldMesh))))))))

(event EventBeginPlay
  ;[1 1 1] BeginPlay
  (bind _returnvalue (UserInterface|CreateWidget "/Game/Blueprints/UI/WBP_Crosshair.WBP_Crosshair_C" (Game|GetPlayerController 0)))
  (bind _output_get (Variables|Default|SetHUD_Widget _returnvalue))
  (UserInterface|Viewport|AddtoViewport _output_get 0))

(event Input|ActionEvents|InputActionInteractLMB
  (params (Key :type Key%20Structure))
  (bind _camera (Variables|Default|GetCamera))
  (bind _itemactor (Variables|Default|GetItemActor))
  (bind _camera_2 (Variables|Default|GetCamera))
  (bind _camera_3 (Variables|Default|GetCamera))
  (bind _itemactor_2 (Variables|Default|GetItemActor))
  (bind _returnvalue (Transformation|GetWorldTransform _camera_2))
  (bind _returnvalue_2 (Transformation|GetWorldTransform _camera_3))
  (bind _returnvalue_3 (Transformation|GetWorldLocation _camera))
  ;[1 1 1] LMB Interact
  (:Pressed
    (if (not (Variables|Default|GetInspecting?))
      ;;[1 1 1] LMB pressed
      ;;;[1 1 1] Draw line from current cam position to target
      (bind (_outhit _returnvalue_4) (Collision|LineTraceByChannel _returnvalue_3 (+ _returnvalue_3 (* (Math|Vector|GetForwardVector _camera) 1000)) "TraceTypeQuery1" false 0 "None"))
      (if _returnvalue_4
        (if (Actor|ActorHasTag (.HitActor (Collision|BreakHitResult _outhit)) "Interactable")
          ;;;[1 1 1] Clear highlight on device
          (CallFunction|ClearHighlight (Variables|Default|GetOldMesh))
          (Variables|Default|SetReturnEndLocationTrs (Transformation|GetActorTransform (.HitActor (Collision|BreakHitResult _outhit))))
          (Variables|Default|SetInspecting? true)
          (Utilities|FlowControl|Sequence
            (:then_0
              ;;;[1 1 1] Timebuffer for sequence to finish
              (Utilities|FlowControl|Delay 0.1)
              ;;;[1 1 1] Hide HUD
              (bind _asbp_inspect_device (Utilities|Casting|CastToBP_Inspect_Device (Variables|/Script/Engine.ChildActorComponent|GetChildActor (Variables|Default|GetItemActor))))
              (Default|HideHUD _asbp_inspect_device)
              ;;;[1 1 1] Pick up animation
              (bind _item_track (Timeline|Timeline_0 PlayFromStart)
                (:Update
                  (Variables|Default|SetStartLocationTrs (Transformation|GetRelativeTransform (Variables|Default|GetItemActor)))
                  (Variables|Default|SetEndLocationTrs (Transformation|GetRelativeTransform (Variables|Default|GetView_Position)))
                  (Transformation|SetRelativeTransform (Variables|Default|GetItemActor) (Math|Transform|Lerp(Transform) (Variables|Default|GetStartLocationTrs) (Variables|Default|GetEndLocationTrs) _item_track) false false))
                (:Finished
                  ;;;[1 1 1] prevent rotation before timeline end
                  (bind _asbp_inspect_device_2 (Utilities|Casting|CastToBP_Inspect_Device (Variables|/Script/Engine.ChildActorComponent|GetChildActor (Variables|Default|GetItemActor))))
                  (Variables|/Game/Blueprints/Interactables/BP_Inspect_Device.BP_Inspect_Device_C|SetinFocus? _asbp_inspect_device_2 true))))
            (:then_1
              ;;;[1 1 1] get pick up item into the blueprint and destroy it in the world
              (ChildActorComponent|SetChildActorClass _itemactor (Utilities|GetClass (.HitActor (Collision|BreakHitResult _outhit))))
              (Transformation|SetRelativeTransform _itemactor (Math|Transform|MakeTransform (Math|Transform|InverseTransformLocation _returnvalue (Transformation|GetActorLocation (.HitActor (Collision|BreakHitResult _outhit)))) (Math|Transform|InverseTransformRotation _returnvalue (Transformation|GetActorRotation (.HitActor (Collision|BreakHitResult _outhit))))) false false)
              (Actor|DestroyActor (.HitActor (Collision|BreakHitResult _outhit)))))))))
  (:Released
    (if (Variables|Default|GetInspecting?)
      ;;[1 1 1] LMB released
      ;;;[1 1 1] reset rotation lock while timeline is active
      (bind _asbp_inspect_device_3 (Utilities|Casting|CastToBP_Inspect_Device (Variables|/Script/Engine.ChildActorComponent|GetChildActor (Variables|Default|GetItemActor))))
      (Variables|/Game/Blueprints/Interactables/BP_Inspect_Device.BP_Inspect_Device_C|SetinFocus? _asbp_inspect_device_3 false)
      ;;;[1 1 1] Show HUD after release
      (Default|ShowHUD _asbp_inspect_device_3)
      ;;;[1 1 1] Reverse pick up animation
      (bind _item_track_2 (Timeline|Timeline_3 Reverse)
        (:Update
          (Variables|Default|SetStartLocationTrs (Transformation|GetRelativeTransform (Variables|Default|GetItemActor)))
          (Variables|Default|SetEndLocationTrs (Transformation|GetRelativeTransform (Variables|Default|GetView_Position)))
          (Transformation|SetRelativeTransform (Variables|Default|GetItemActor) (Math|Transform|Lerp(Transform) (Variables|Default|GetStartLocationTrs) (Variables|Default|GetEndLocationTrs) _item_track_2) false false))
        (:Finished
          ;;;[1 1 1] Spawns the held item back into the world
          (bind _returnvalue_5 (Game|SpawnActorfromClass (Variables|/Script/Engine.ChildActorComponent|GetChildActorClass (Variables|Default|GetItemActor)) (Math|Transform|MakeTransform (Math|Transform|TransformLocation _returnvalue_2 (Variables|/Script/Engine.SceneComponent|GetRelativeLocation _itemactor_2)) (Math|Transform|TransformRotation _returnvalue_2 (Variables|/Script/Engine.SceneComponent|GetRelativeRotation _itemactor_2))) "Undefined" 0 0))
          (Variables|Default|SetPlacedItem _returnvalue_5)
          ;;;[1 1 1] removes item holding
          (ChildActorComponent|SetChildActorClass (Variables|Default|GetItemActor) 0)
          ;;;[1 1 1] Sets the item transform as start location
          (Variables|Default|SetReturnStartLocationTrs (Transformation|GetActorTransform (Variables|Default|GetPlacedItem)))
          ;;;[1 1 1] Place down animation
          (bind _return_location_track (Timeline|Reset%20item%20location PlayFromStart)
            (:Update
              (Transformation|SetActorTransform (Variables|Default|GetPlacedItem) (Math|Transform|Lerp(Transform) (Variables|Default|GetReturnStartLocationTrs) (Variables|Default|GetReturnEndLocationTrs) _return_location_track)))
            (:Finished
              (Variables|Default|SetInspecting? false))))))))

(event Input|ActionEvents|InputActionInspectRMB
  (params (Key :type Key%20Structure))
  ;[1 1 1] RMB Inspect item
  (:Pressed
    (bind _asbp_inspect_device (Utilities|Casting|CastToBP_Inspect_Device (Variables|/Script/Engine.ChildActorComponent|GetChildActor (Variables|Default|GetItemActor))))
    (Default|StartInspect _asbp_inspect_device self)))

(event Input|AxisEvents|InputAxisMoveForward
  (params (AxisValue :type Float%20%28single-precision%29))
  ;[1 1 1] Movement
  (Pawn|Input|AddMovementInput (Transformation|GetActorForwardVector) AxisValue false))

(event Input|AxisEvents|InputAxisMoveRight
  (params (AxisValue :type Float%20%28single-precision%29))
  ;[1 1 1] Movement
  (Pawn|Input|AddMovementInput (Transformation|GetActorRightVector) AxisValue false))

(event Input|AxisEvents|InputAxisLookUp
  (params (AxisValue :type Float%20%28single-precision%29))
  ;[1 1 1] Movement
  (Pawn|Input|AddControllerPitchInput (* AxisValue (Variables|Default|GetMouseSpeed))))

(event Input|AxisEvents|InputAxisTurn
  (params (AxisValue :type Float%20%28single-precision%29))
  ;[1 1 1] Movement
  (Pawn|Input|AddControllerYawInput (* AxisValue (Variables|Default|GetMouseSpeed))))

(fn ConstructionScript)

(fn ClearHighlight
  (params (MeshToClear :type Primitive%20Component%20Object%20Reference))
  (Rendering|SetRenderCustomDepth MeshToClear false)
  (Rendering|SetCustomDepthStencilValue MeshToClear 0))