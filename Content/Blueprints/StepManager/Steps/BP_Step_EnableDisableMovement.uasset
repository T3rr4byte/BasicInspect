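; A step-manager step that turns player movement on or off, based on its Enable flag.
; Beginning the step applies the flag and finishes immediately; skipping applies it without finishing, and undoing applies the opposite.
; The helper casts the player pawn to BP_RW1Pawn, then switches between walking with game-only input and disabled movement with UI-only input and locked mouse.
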(event EventBeginStep
  (CallFunction|EnableDisableMovement (Variables|Default|GetEnable))
  (CallFunction|StepFinished))

(event EventSkipStep
  (CallFunction|EnableDisableMovement (Variables|Default|GetEnable)))

(event EventUndoStep
  (CallFunction|EnableDisableMovement (not (Variables|Default|GetEnable))))

(fn ConstructionScript
  (|CallParentFunction))

(fn EnableDisableMovement
  (params (Enable :type Boolean))
  (bind _returnvalue (Game|GetPlayerController 0))
  (bind _asbp_rw1pawn (Utilities|Casting|CastToBP_RW1Pawn (Game|Player|GetPlayerPawn 0))
    (:then
      (if Enable
        ;[1 1 1] Enable/disable keyboard movement
        (Pawn|Components|CharacterMovement|SetMovementMode (Variables|/Script/Engine.Character|GetCharacterMovement _asbp_rw1pawn) "MOVE_Walking" 0)
        ;[1 1 1] Enable/disable mouse movement
        (Input|SetInputModeGameOnly _returnvalue)
        (else
          (Pawn|Components|CharacterMovement|DisableMovement (Variables|/Script/Engine.Character|GetCharacterMovement _asbp_rw1pawn))
          (Input|SetInputModeUIOnly _returnvalue 0 "LockAlways"))))
    (:CastFailed
      (Development|PrintString "Failed to get BP_RW1Pawn!"))))