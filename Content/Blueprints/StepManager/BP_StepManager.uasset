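; BP_StepManager runs an ordered list of step actors one after another as a linear sequence.
; Its construction script hands each step a reference back to the manager.
; It optionally starts on BeginPlay, begins the current step, and advances the counter when the active step reports StepFinished.
; Finish calls from non-active steps are rejected with a debug print, and the flow simply stops after the last step.
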(event Custom|Start
  ;[1 1 1] Start - Starting the overall flow
  (if (Utilities|Array|IsValidIndex (Variables|Default|GetSteps))
    (CallFunction|StartStep)
    (else
      (Development|PrintString "Attempted to start step manager but no valid steps added!"))))

(event Custom|StepFinished
  (params (Step :type BP%20Step%20Base%20Object%20Reference))
  ;[1 1 1] StepFinished - Called from BP_Step
  (if (!= (Variables|Default|GetActiveStep) Step)
    (Development|PrintString "Step finished called but it's not the active step!")
    (else
      (Math|Integer|IncrementInt (Variables|Default|GetStepCounter)
        (:%20%20
          (CallFunction|StartStep))))))

(event Custom|StartStep
  (bind _stepcounter (Variables|Default|GetStepCounter))
  (bind _steps (Variables|Default|GetSteps))
  (bind _output (Utilities|Array|Get(acopy) _steps _stepcounter))
  ;[1 1 1] StartStep - Starts the step at the current StepCounter
  (if (Utilities|Array|IsValidIndex (Variables|Default|GetSteps) (Variables|Default|GetStepCounter))
    (Development|PrintString (Utilities|String|Append "Starting Step: " (Utilities|GetDisplayName _output)) true true "(R=0.000000,G=0.660000,B=1.000000,A=1.000000)" 1e+01)
    (bind _output_get (Variables|Default|SetActiveStep _output))
    (Default|BeginStep _output_get)))

(event EventBeginPlay
  ;[1 1 1] BeginPlay
  (if (Variables|Default|GetStartOnBeginPlay)
    (CallFunction|Start)))

(fn ConstructionScript
  (for _array_element (Variables|Default|GetSteps)
    (Variables|/Game/Blueprints/StepManager/BP_StepBase.BP_StepBase_C|SetStepManager _array_element self)))