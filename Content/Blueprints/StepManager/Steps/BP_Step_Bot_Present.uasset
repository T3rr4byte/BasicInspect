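; BP_Step_Bot_Present is a step Blueprint that reveals a character, presumably the bot, by playing a level sequence.
; It hides the Character and its child components on BeginPlay, then shows them when the step begins.
; BeginStep creates and plays a player for the provided Sequence, waits out its duration with a Delay, then calls StepFinished.
; SkipStep and UndoStep are empty.
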(event EventBeginStep
  ;[1 1 1] Set visibility
  (Rendering|SetVisibility (Variables|/Script/Engine.Actor|GetRootComponent (Variables|Default|GetCharacter)) true true)
  ;[1 1 1] Play the provided sequence
  (bind _outactor (Sequencer|Player|CreateLevelSequencePlayer (Variables|Default|GetSequence)))
  (Sequencer|Player|Play (Variables|/Script/LevelSequence.LevelSequenceActor|GetSequencePlayer _outactor) :!class /Script/MovieScene.MovieSceneSequencePlayer)
  (Utilities|FlowControl|Delay (Class|TimeManagementBlueprintLibrary|ToSeconds(QualifiedFrameTime) (Media|MediaPlayer|GetDuration (Variables|/Script/LevelSequence.LevelSequenceActor|GetSequencePlayer _outactor))))
  (CallFunction|StepFinished))

(event EventSkipStep)

(event EventUndoStep)

(event EventBeginPlay
  ;[1 1 1] Set visibility
  (Rendering|SetVisibility (Variables|/Script/Engine.Actor|GetRootComponent (Variables|Default|GetCharacter)) false true))

(fn ConstructionScript
  (|CallParentFunction))