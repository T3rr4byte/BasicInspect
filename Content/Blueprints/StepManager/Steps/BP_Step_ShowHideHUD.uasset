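; BP_Step_ShowHideHUD is a step manager step that shows or hides the crosshair HUD according to its Show flag.
; On BeginStep it calls CrosshairShowHide and finishes immediately.
; Showing creates a WBP_Crosshair for player 0, stores it in HUDWidget and adds it to the viewport, while hiding removes that stored widget.
; SkipStep and UndoStep do nothing.
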(event EventBeginStep
  (CallFunction|CrosshairShowHide (Variables|Default|GetShow?))
  (CallFunction|StepFinished))

(event EventSkipStep)

(event EventUndoStep)

(fn ConstructionScript
  (|CallParentFunction))

(fn CrosshairShowHide
  (params (Show :type Boolean))
  (if Show
    (bind _returnvalue (UserInterface|CreateWidget "/Game/Blueprints/UI/WBP_Crosshair.WBP_Crosshair_C" (Game|GetPlayerController 0)))
    (bind _output_get (Variables|Default|SetHUD_Widget _returnvalue))
    (UserInterface|Viewport|AddtoViewport _output_get 0)
    (else
      (Widget|RemovefromParent (Variables|Default|GetHUD_Widget)))))