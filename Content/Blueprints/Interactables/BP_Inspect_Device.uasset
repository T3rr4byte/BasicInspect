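; Inspectable device actor that the player can rotate with the mouse while examining it.
; StartInspect moves input from the inspecting pawn to this actor and hides the crosshair widget.
; While InFocus is set, mouse axes rotate the device mesh and the pawn's ItemActor together, preventing a rotation jump on release.
; Releasing RMB hands input back, while releasing LMB also clears focus, calls the pawn's EndInteract and restores the crosshair.
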(event Custom|Start%20Inspect
  (params (Inspector :type Pawn%20Object%20Reference))
  (bind _returnvalue (Game|GetPlayerController 0))
  ;[1 1 1] start inspect RMB
  (bind _output_get (Variables|Default|SetInspector Inspector))
  (Input|DisableInput _output_get _returnvalue)
  (Input|EnableInput _returnvalue)
  (CallFunction|HideHUD))

(event Custom|Hide%20HUD
  (bind _crosshair_wbp (Variables|Default|GetCrosshair_WBP))
  ;[1 1 1] Hide HUD
  (Utilities|IsValid _crosshair_wbp
    (:Is%20Valid
      (Widget|SetRenderOpacity _crosshair_wbp 0.0))
    (:Is%20Not%20Valid
      (Development|PrintString "No HUD widget available!"))))

(event Custom|Show%20HUD
  (bind _crosshair_wbp (Variables|Default|GetCrosshair_WBP))
  ;[1 1 1] Show HUD
  (Utilities|IsValid _crosshair_wbp
    (:Is%20Valid
      (Widget|SetRenderOpacity _crosshair_wbp 1.0))
    (:Is%20Not%20Valid
      (Development|PrintString "No HUD widget available!"))))

(event EventBeginPlay
  ;[1 1 1] Set UI for later use
  (bind _foundwidgets (Widget|GetAllWidgetsOfClass "/Game/Blueprints/UI/WBP_Crosshair.WBP_Crosshair_C" true))
  (Variables|Default|SetCrosshair_WBP (Utilities|Array|Get(acopy) _foundwidgets))
  ;[1 1 1] Set pawn item actor used in mouse x/y movement
  (bind _asbp_rw1pawn (Utilities|Casting|CastToBP_RW1Pawn (Game|GetPlayerCharacter 0))
    (:then
      (Variables|Default|SetPawnItemActor _asbp_rw1pawn))
    (:CastFailed
      (Development|PrintString "BP_Interactable: Cast to Pawn failed!"))))

(event Input|ActionEvents|InputActionInspectRMB
  (params (Key :type Key%20Structure :default "None"))
  (bind _returnvalue (Game|GetPlayerController 0))
  ;[1 1 1] stop inspecting RMB
  (:Released
    (Input|DisableInput _returnvalue)
    (Input|EnableInput (Variables|Default|GetInspector) _returnvalue)))

(event Input|ActionEvents|InputActionInteractLMB
  (params (Key :type Key%20Structure :default "None"))
  (bind _returnvalue (Game|GetPlayerController 0))
  (bind _inspector (Variables|Default|GetInspector))
  ;[1 1 1] stop interacting LMB
  (:Released
    (Variables|Default|SetinFocus? false)
    (Input|DisableInput _returnvalue)
    (Input|EnableInput _inspector _returnvalue)
    (bind _asbp_rw1pawn (Utilities|Casting|CastToBP_RW1Pawn _inspector))
    (Default|EndInteract _asbp_rw1pawn)
    (CallFunction|ShowHUD)))

(event Input|MouseEvents|MouseX
  (params (AxisValue :type Float%20%28single-precision%29))
  (bind _returnvalue (* AxisValue -1.0))
  (bind _pawnitemactor (Variables|Default|GetPawnItemActor))
  (bind _itemactor (Variables|/Game/Blueprints/Base/BP_RW1Pawn.BP_RW1Pawn_C|GetItemActor _pawnitemactor))
  ;[1 1 1] Mouse X movement
  ;;[1 1 1] prevent rotation before timeline end
  (if (Variables|Default|GetinFocus?)
    ;;[1 1 1] set interactable device rotation
    (Transformation|SetRelativeRotation (Variables|Default|GetSM_Device) (Math|Rotator|CombineRotators (Variables|/Script/Engine.SceneComponent|GetRelativeRotation (Variables|Default|GetSM_Device)) (Math|Rotator|MakeRotator 0.0 0.0 _returnvalue)) false false)
    ;;[1 1 1] Set pawn child actor rotation (prevent roration jump on button release)
    (Transformation|SetRelativeRotation _itemactor (Math|Rotator|CombineRotators (Variables|/Script/Engine.SceneComponent|GetRelativeRotation _itemactor) (Math|Rotator|MakeRotator 0.0 0.0 _returnvalue)) false false)))

(event Input|MouseEvents|MouseY
  (params (AxisValue :type Float%20%28single-precision%29))
  (bind _returnvalue (* AxisValue -1.0))
  (bind _pawnitemactor (Variables|Default|GetPawnItemActor))
  (bind _itemactor (Variables|/Game/Blueprints/Base/BP_RW1Pawn.BP_RW1Pawn_C|GetItemActor _pawnitemactor))
  ;[1 1 1] Mouse Y movement
  ;;[1 1 1] prevent rotation before timeline end
  (if (Variables|Default|GetinFocus?)
    ;;[1 1 1] Set interactable device rotation
    (Transformation|SetRelativeRotation (Variables|Default|GetSM_Device) (Math|Rotator|CombineRotators (Variables|/Script/Engine.SceneComponent|GetRelativeRotation (Variables|Default|GetSM_Device)) (Math|Rotator|MakeRotator 0.0 _returnvalue 0.0)) false false)
    ;;[1 1 1] Set pawn child actor rotation (prevent roration jump on button release)
    (Transformation|SetRelativeRotation _itemactor (Math|Rotator|CombineRotators (Variables|/Script/Engine.SceneComponent|GetRelativeRotation _itemactor) (Math|Rotator|MakeRotator 0.0 _returnvalue 0.0)) false false)))

(fn ConstructionScript)

(fn NewFunction0
  (bind _asbp_rw1pawn (Utilities|Casting|CastToBP_RW1Pawn (Game|GetPlayerCharacter 0)))
  (Transformation|SetRelativeRotation (Variables|/Game/Blueprints/Base/BP_RW1Pawn.BP_RW1Pawn_C|GetItemActor _asbp_rw1pawn) (Variables|/Script/Engine.SceneComponent|GetRelativeRotation (Variables|Default|GetSM_Device)) false false))